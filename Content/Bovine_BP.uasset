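; Bovine anatomy actor for a VR game, with skeleton meshes and separate heart, kidney, stomach and lung organs.
; On BeginPlay it caches the player's VR pawn, stopping if the cast fails.
; It then builds the bone mesh list by gathering all static mesh components and removing the four organs.
; The graph only performs this setup, with no tick, overlap or construction logic.
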(event EventBeginPlay
  (bind _asvrpawn (Utilities|Casting|CastToVRPawn (Game|Player|GetPlayerPawn 0)))
  (Variables|Default|SetVRPawn _asvrpawn)
  (bind _output_get (Variables|Default|SetBone_StaticMeshes (Actor|GetComponentsByClass "/Script/Engine.StaticMeshComponent")))
  (Utilities|Array|RemoveItem _output_get (Variables|Default|GetHeart))
  (Utilities|Array|RemoveItem _output_get (Variables|Default|GetKidney))
  (Utilities|Array|RemoveItem _output_get (Variables|Default|GetStomach))
  (Utilities|Array|RemoveItem _output_get (Variables|Default|GetBovine_Lungs)))

(event Collision|EventActorBeginOverlap
  (params (OtherActor :type Actor%20Object%20Reference)))

(event EventTick
  (params (DeltaSeconds :type Float%20%28single-precision%29)))

(fn ConstructionScript)